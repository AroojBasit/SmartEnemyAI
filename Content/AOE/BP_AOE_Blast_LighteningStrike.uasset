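; Lightning strike variant of an AOE blast that warns with a ground decal before it goes off.
; On BeginPlay it runs the parent logic, calls MoveToFloor on the attack target and spawns the decal at the actor's location.
; After a configurable delay it calls Trigger and destroys the decal.
; An unconnected downward trace that would snap the actor to the floor under the target remains in the graph but never runs.
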(event `self.ReceiveBeginPlay`
  (`parent.ReceiveBeginPlay`)
  (`self.MoveToFloor` (`self.AttackTarget`))
  (bind _returnvalue (`GameplayStatics.SpawnDecalAtLocation` (`self.Decal Material`) (25.0 256.0 256.0) (`self.K2_GetActorLocation`)))
  (`KismetSystemLibrary.Delay` (`self.DelayBeforeStrike`))
  (`self.Trigger`)
  (`/Engine/EditorBlueprintResources/StandardMacros.IsValid` _returnvalue
    (:`Is Valid`
      (`ActorComponent.K2_DestroyComponent` _returnvalue))))

(fn `UserConstructionScript`
  (`parent.UserConstructionScript`))