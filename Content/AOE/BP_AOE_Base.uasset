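; BP_AOE_Base is a base area-of-effect actor that finds pawns within a radius, firing on BeginPlay or when Trigger is called.
; Trigger runs a sphere overlap at its location, optionally ignoring the instigator and drawing a debug sphere, then sets a short lifespan.
; Each overlapped actor is passed to the OnAOEOverlapActor dispatcher, keeping effects separate from detection.
; A MoveToFloor helper snaps the AOE to the floor beneath a given actor.
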(event `self.ReceiveBeginPlay`
  (if (`self.TriggerOnBeganPlay`)
    (`self.Trigger`)))

(event `Trigger`
  (`self.SpawnAOESphere`)
  (`self.SetLifeSpan` 2.0))

(event `SpawnAOESphere`
  (if (`self.DrawDebugSphere`)
    (`KismetSystemLibrary.DrawDebugSphere` (`self.K2_GetActorLocation`) (`self.Radius`) 12 (struct :`R` 1.0 :`B` 0.891643 :`A` 1.0) 2.0 1.0))
  (bind _outactors (`KismetSystemLibrary.SphereOverlapActors` (`self.K2_GetActorLocation`) (`self.Radius`) (`|MakeArray` "ObjectTypeQuery3" :!type "EObjectTypeQuery Enum") null (select `bool` (`self.IgnoreInstigator`) :`true` (`|MakeArray` (`self.GetInstigator`) :!type "Actor Object Reference"))))
  (for _array_element _outactors
    ;[1 1 1] Separation of Concerns
    (`self.OnAOEOverlapActor` _array_element)))

(event `MoveToFloor`
  (params (Actor :type "Actor Object Reference"))
  (bind _returnvalue (`self.K2_GetActorLocation` Actor))
  (bind (_outhit _returnvalue_2) (`KismetSystemLibrary.LineTraceSingle` _returnvalue (+ _returnvalue (1.0 1.0 -1000.0)) "TraceTypeQuery1" false (`|MakeArray` Actor)))
  (if _returnvalue_2
    (`self.K2_SetActorLocation` (`.Location` (`GameplayStatics.BreakHitResult` _outhit)))))

(fn `UserConstructionScript`)