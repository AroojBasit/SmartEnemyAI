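; BP_Enemy_Meele is a sword-wielding melee enemy, built on a parent class, with short-range, jumping long-range, spin and ground-smash attacks.
; Each attack event hands a montage and damage info to the Attacks component.
; Equip and unequip montages use notifies to spawn and socket or destroy the sword, calling equipped or unequipped callbacks on completion.
; It also supplies ideal attack and defend ranges and caches mesh rotation at construction.
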(event `self.ReceiveBeginPlay`
  (`parent.ReceiveBeginPlay`))

(event `ShortRangeAttack`
  (params (AttackTarget :type "Actor Object Reference"))
  ;[1 1 1] Attacks
  (`/Game/Attacks/BPC_Attacks.PrimaryMeleeAttack` (`self.Attacks`) (make `/Game/Attacks/S_AttackInfo` AttackTarget "/Game/Animations/Melee/Montage/Montage_SwordSlash.Montage_SwordSlash" (make `/Game/DamageSystem/S_DamageInfo` 10.0 "NewEnumerator1" "NewEnumerator1" false true true)) 20.0 200.0))

(event `LongRangeAttack`
  (params (AttackTarget :type "Actor Object Reference"))
  ;[1 1 1] Attacks
  (`/Game/Attacks/BPC_Attacks.LongRangeMeleeAttack` (`self.Attacks`) (make `/Game/Attacks/S_AttackInfo` AttackTarget "/Game/Animations/Melee/Montage/Montage_MeleeJumpAttack.Montage_MeleeJumpAttack" (make `/Game/DamageSystem/S_DamageInfo` 10.0 "NewEnumerator1" "NewEnumerator1" false true true)) 20.0 200.0 2.0))

(event `SpinAttack`
  (params (AttackTarget :type "Actor Object Reference"))
  ;[1 1 1] Attacks
  (`/Game/Attacks/BPC_Attacks.SpinMeleeAttack` (`self.Attacks`) (make `/Game/Attacks/S_AttackInfo` AttackTarget "/Game/Animations/Melee/Montage/Montage_SwordSpinAttack.Montage_SwordSpinAttack" (make `/Game/DamageSystem/S_DamageInfo` 1.0 "NewEnumerator1" "NewEnumerator1" false true)) 20.0 200.0 300.0))

(event `GroundSmashAttack`
  (params (AttackTarget :type "Actor Object Reference"))
  ;[1 1 1] Attacks
  (`/Game/Attacks/BPC_Attacks.GroundSmash` (`self.Attacks`) (make `/Game/Attacks/S_AttackInfo` AttackTarget "/Game/Animations/Melee/Montage/Montage_MeleeGroundSmash.Montage_MeleeGroundSmash" (make `/Game/DamageSystem/S_DamageInfo` 25.0 "NewEnumerator3" "NewEnumerator1")) 300.0))

(event `/Game/Enemies/AI/BPI_EnemyAI.EquipWeapon`
  ;[1 1 1] Weapon
  (bind _notifyname (`|PlayMontage` (`self.Mesh`) "/Game/Animations/Melee/Montage/Montage_UnsheathSword.Montage_UnsheathSword")
    (:`OnCompleted`
      (`self.OnWeaponEquiped`))
    (:`OnNotifyBegin`
      (switch `name` _notifyname
        (:`HoldSword`
          (bind _returnvalue (`|SpawnActorFromClass` "/Game/Weapon/BP_Weapon_Sword.BP_Weapon_Sword_C" (`self.GetTransform`) "Undefined" "MultiplyWithRoot" null null))
          (bind _output_get (set `self.WeaponActor` _returnvalue))
          (`self.K2_AttachToComponent` _output_get (`self.Mesh`) "hand_r_sword_socket" "SnapToTarget" "SnapToTarget" "SnapToTarget" true)
          (set `self.IsWeaponEquiped` true))))))

(event `/Game/Enemies/AI/BPI_EnemyAI.UnequipWeapon`
  ;[1 1 1] Weapon
  (bind _notifyname (`|PlayMontage` (`self.Mesh`) "/Game/Animations/Melee/Montage/Montage_SheathSword.Montage_SheathSword")
    (:`OnCompleted`
      (`self.OnWeaponUnequiped`))
    (:`OnNotifyBegin`
      (switch `name` _notifyname
        (:`DropSword`
          (`self.K2_DestroyActor` (`self.WeaponActor`))
          (set `self.IsWeaponEquiped` false))))))

(fn `GetIdealRange`
  (returns (AttackRadius :type "Float (double-precision)") (DefendRadius :type "Float (double-precision)"))
  (return 200.0 400.0))

(fn `UserConstructionScript`
  (`parent.UserConstructionScript`)
  (set `self.MeshRotationBeforeSpin` (`SceneComponent.RelativeRotation` (`self.Mesh`))))