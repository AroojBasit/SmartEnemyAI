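; BP_PatrolRoute is a spline-based patrol path for enemy AI to follow.
; IncrementPatrolRoute advances a point index by a direction value, flipping direction at either end so the route ping-pongs.
; GetSplinePointAsWorldPosition returns the current spline point's world location as the movement target.
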(event `IncrementPatrolRoute`
  (bind _output_get (set `self.PartolIndex` (+ (`self.PartolIndex`) (`self.Direction`))))
  (if (== _output_get (- (`SplineComponent.GetNumberOfSplinePoints` (`self.PatrolRoute`)) 1))
    (set `self.Direction` -1)
    (elif (== (`self.PartolIndex`) 0)
      (set `self.Direction` 1))))

(fn `GetSplinePointAsWorldPosition`
  (returns (Location :type "Vector Structure"))
  (return (`SplineComponent.GetLocationAtSplinePoint` (`self.PatrolRoute`) (`self.PartolIndex`) "World")))

(fn `UserConstructionScript`)