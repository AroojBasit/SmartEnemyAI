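; Ranged enemy character that spawns a rifle on begin play and attaches it to a hand socket on its mesh.
; ShootWeapon passes an attack struct with target, fire montage and fixed damage, plus the rifle, to the Attacks component's ranged attack.
; Helper functions map movement speed states to walk speed, supply fixed attack and defend ranges, and report whether it is attacking.
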(event `self.ReceiveBeginPlay`
  (`parent.ReceiveBeginPlay`)
  (`self.EquipWeapon`))

(event `/Game/Enemies/AI/BPI_EnemyAI.EquipWeapon`
  (bind _returnvalue (`|SpawnActorFromClass` "/Game/Weapon/BP_Weapon_Rifle.BP_Weapon_Rifle_C" (`self.GetTransform`) "Undefined" "MultiplyWithRoot" null null))
  (bind _output_get (set `self.WeaponActor` _returnvalue))
  (`self.K2_AttachToComponent` _output_get (`self.Mesh`) "hand_r_rifle_socket" "SnapToTarget" "SnapToTarget" "SnapToTarget" true)
  (set `self.IsWeaponEquiped` true)
  (`self.OnWeaponEquiped`))

(event `ShootWeapon`
  (params (AttackTarget :type "Actor Object Reference"))
  (`/Game/Attacks/BPC_Attacks.RangedAttack` (`self.Attacks`) (make `/Game/Attacks/S_AttackInfo` AttackTarget "/Game/Animations/Rifle/Montage_RifleFire.Montage_RifleFire" (make `/Game/DamageSystem/S_DamageInfo` 15.0 "NewEnumerator2" "NewEnumerator0" false true)) (`self.WeaponActor`)))

(fn `GetIdealRange`
  (returns (AttackRadius :type "Float (double-precision)") (DefendRadius :type "Float (double-precision)"))
  (return 600.0 600.0))

(fn `IsAttacking`
  (returns (Attacking :type Boolean))
  (return (`self.Attacking`)))

(fn `SetMovementSpeed`
  (params (Speed :type "/Game/Enemies/AI/Enums/E_MovementSpeed Enum" :default "NewEnumerator0"))
  (returns (SpeedValue :type "Float (double-precision)"))
  (bind _output_get (set `CharacterMovementComponent.MaxWalkSpeed` (select `/Game/Enemies/AI/Enums/E_MovementSpeed` Speed :`NewEnumerator1` 200.0 :`NewEnumerator2` 300.0 :`NewEnumerator3` 500.0 :!type "Float (single-precision)") (`self.CharacterMovement`)))
  (return _output_get))

(fn `UserConstructionScript`
  (`parent.UserConstructionScript`))